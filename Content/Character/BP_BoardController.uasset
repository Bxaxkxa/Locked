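; BP_BoardController is a player controller that sets up the board game's player UI.
; On BeginPlay it creates and stores turn input, action indicator, duel option, duel and health info widgets, then adds them to the viewport after a short delay.
; A separate AddDisplay event creates and shows a turn display, only on the local player controller.
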(event Custom|AddDisplay
  (CallFunction|AddTurnDisplaySomething))

(event Custom|AddTurnDisplaySomething
  (if (Pawn|IsLocalPlayerController)
    (bind _returnvalue (UserInterface|CreateWidget "/Game/UMG/Widget/TurnDisplay.TurnDisplay_C"))
    (UserInterface|Viewport|AddtoViewport _returnvalue 0)))

(event Custom|CreatePlayerInputWidget_Event
  (bind _self self)
  (bind _self_2 self)
  (Utilities|FlowControl|Sequence
    (:then_0
      (bind _returnvalue (UserInterface|CreateWidget "/Game/UMG/Widget/BP_PlayerTurnInput.BP_PlayerTurnInput_C" _self))
      (bind _output_get (Variables|Default|SetActionUIWidget _self _returnvalue))
      (bind _returnvalue_2 (UserInterface|CreateWidget "/Game/UMG/Widget/BP_ActionIndicatorLayout.BP_ActionIndicatorLayout_C" _self_2))
      (bind _output_get_2 (Variables|Default|SetActionIndicatorWidget _self_2 _returnvalue_2))
      (bind _returnvalue_3 (UserInterface|CreateWidget "/Game/UMG/Widget/BP_DuelOption.BP_DuelOption_C" self))
      (bind _output_get_3 (Variables|Default|SetDuelOptionWidget _returnvalue_3))
      (bind _returnvalue_4 (UserInterface|CreateWidget "/Game/UMG/Widget/BP_DuelWidget.BP_DuelWidget_C"))
      (bind _output_get_4 (Variables|Default|SetDuelWidget _returnvalue_4))
      (bind _returnvalue_5 (UserInterface|CreateWidget "/Game/UMG/Widget/BP_PlayerHealthInfo.BP_PlayerHealthInfo_C"))
      (bind _output_get_5 (Variables|Default|SetPlayerHealthInfo _returnvalue_5)))
    (:then_1
      (Utilities|FlowControl|Delay 0.2)
      (UserInterface|Viewport|AddtoViewport _output_get 0)
      (UserInterface|Viewport|AddtoViewport _output_get_2 1)
      (UserInterface|Viewport|AddtoViewport _output_get_3 1)
      (UserInterface|Viewport|AddtoViewport _output_get_4 0)
      (UserInterface|Viewport|AddtoViewport _output_get_5 0))))

(event EventBeginPlay
  (CallFunction|CreatePlayerInputWidgetEvent))

(event EventTick
  (params (DeltaSeconds :type Float%20%28single-precision%29)))

(fn ConstructionScript)