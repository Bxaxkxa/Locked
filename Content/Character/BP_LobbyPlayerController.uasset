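; Lobby player controller that sets game-only input on BeginPlay and handles leaving the session when kicked or when the lobby closes.
; Both exit events destroy the session, then open MainMenu with an option string naming the reason.
; AddWidgetLayout shows a non-interactive action indicator after a short delay, but its only call here, alongside host settings UI, is disconnected.
; Tick scans all user widgets and prints whichever has user focus as debug output.
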(event Custom|LeaveClosedLobby
  (|DestroySession self
    (:OnSuccess
      (Game|OpenLevel(byName) "MainMenu" true "LobbyClosed"))))

(event Custom|KickedFromGame
  (|DestroySession self
    (:OnSuccess
      (Game|OpenLevel(byName) "MainMenu" true "Kicked"))))

(event Custom|AddWidgetLayout
  (bind _self self)
  (bind _returnvalue (UserInterface|CreateWidget "/Game/UMG/Widget/BP_ActionIndicatorLayout.BP_ActionIndicatorLayout_C" _self))
  (bind _output_get (Variables|Default|SetActionIndicatorWidget _self _returnvalue))
  (Utilities|FlowControl|Delay 0.2)
  (UserInterface|Viewport|AddtoViewport _output_get 1)
  (Widget|SetVisibility _output_get "HitTestInvisible"))

(event EventBeginPlay
  (Input|SetInputModeGameOnly self))

(event EventTick
  (params (DeltaSeconds :type Float%20%28single-precision%29))
  (bind _foundwidgets (Widget|GetAllWidgetsOfClass "/Script/UMG.UserWidget" false))
  (bind _array_element (Utilities|Array|ForEachLoopwithBreak _foundwidgets)
    (:LoopBody
      (if (Class|Widget|HasUserFocus _array_element self)
        (Development|PrintString (Utilities|GetDisplayName _array_element) true true "(R=0.000000,G=0.660000,B=1.000000,A=1.000000)" 0.0)))))

(fn ConstructionScript)