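; Lobby game mode that handles the host closing the lobby.
; HostLeaveLobby loops over every player controller after the host's and calls LeaveClosedLobby on each BP_LobbyPlayerController.
; It then destroys the session through player 0 and, on success, opens the MainMenu level.
; A player-count check that would skip the loop is left unconnected.
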(event Custom|HostLeaveLobby
  (bind _returnvalue (Class|GameModeBase|GetNumPlayers))
  (for _index (range 2 _returnvalue)
    (bind _asbp_lobby_player_controller (Utilities|Casting|CastToBP_LobbyPlayerController (Game|GetPlayerController (- _index 1))))
    (Default|LeaveClosedLobby _asbp_lobby_player_controller))
  (|DestroySession (Game|GetPlayerController 0)
    (:OnSuccess
      (Game|OpenLevel(byName) "MainMenu"))))

(event EventBeginPlay)

(event EventTick
  (params (DeltaSeconds :type Float%20%28single-precision%29)))

(fn ConstructionScript)